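; BP_NPC is an interactable NPC that shows dialogue lines one at a time on the player's WDGameplay widget.
; Each Interact increments TalkIndex and picks Dialogue1 or Dialogue2 by NPCIndex, hiding the interaction prompt while text shows.
; Past the last line it hides the dialogue and resets TalkIndex to -1.
; Both branches bound the index by Dialogue1's length, even when reading Dialogue2.
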(event `StartDialogue`
  (`/Game/Blueprints/WD_Gameplay.DisplayDialogue` (`/Game/Blueprints/BP_Player.WD_Gameplay` (`self.Player`)))
  (`/Game/Blueprints/WD_Gameplay.UndisplayInteractionText` (`/Game/Blueprints/BP_Player.WD_Gameplay` (`self.Player`))))

(event `self.ReceiveBeginPlay`
  (bind _asbp_player (cast `/Game/Blueprints/BP_Player` (`GameplayStatics.GetPlayerCharacter` 0)))
  (set `self.Player` _asbp_player))

(event `FinishDialogue`
  (`/Game/Blueprints/WD_Gameplay.UndisplayDialogue` (`/Game/Blueprints/BP_Player.WD_Gameplay` (`self.Player`)))
  (set `self.TalkIndex` -1))

(event `/Game/I_InteractableObjectsInterface.Interact`
  (`/Engine/EditorBlueprintResources/StandardMacros.IncrementInt` (`self.TalkIndex`)
    (:`  `
      (switch `int` (`self.NPC_Index`)
        (:`1`
          (if (< (`self.TalkIndex`) (`KismetArrayLibrary.Array_Length` (`self.Dialogue#1`)))
            (`self.StartDialogue`)
            (set `TextBlock.Text` (`KismetTextLibrary.Conv_StringToText` (`|GetArrayItem` (`self.Dialogue#1`) (`self.TalkIndex`))) (`/Game/Blueprints/WD_Gameplay.DialogueText` (`/Game/Blueprints/BP_Player.WD_Gameplay` (`self.Player`))))
            (else
              (`self.FinishDialogue`))))
        (:`2`
          (if (< (`self.TalkIndex`) (`KismetArrayLibrary.Array_Length` (`self.Dialogue#1`)))
            (`self.StartDialogue`)
            (set `TextBlock.Text` (`KismetTextLibrary.Conv_StringToText` (`|GetArrayItem` (`self.Dialogue#2`) (`self.TalkIndex`))) (`/Game/Blueprints/WD_Gameplay.DialogueText` (`/Game/Blueprints/BP_Player.WD_Gameplay` (`self.Player`))))
            (else
              (`self.FinishDialogue`))))))))

(fn `UserConstructionScript`)