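; BP_Totem is a totem actor that can move under physics only while a specific companion is the active character.
; On BeginPlay it caches BP_Player and binds to its character-swapped event.
; Each swap checks the player's current character, enabling physics simulation on the Totem component for Companion 1 and disabling it for the player and the other two companions.
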(event `self.ReceiveBeginPlay`
  (bind _asbp_player (cast `/Game/Blueprints/BP_Player` (`GameplayStatics.GetPlayerCharacter` 0)))
  (set `self.Player` _asbp_player)
  (add `/Game/Blueprints/BP_Player.CharacterSwapped` (`self.Player`) (delegate `SetTotemMovement`)))

(event `SetTotemMovement`
  (bind _totem (`self.Totem`))
  (switch `/Game/CurrentCharacter` (`/Game/Blueprints/BP_Player.CurrentCharacter` (`self.Player`))
    (:`NewEnumerator0`
      (`PrimitiveComponent.SetSimulatePhysics` _totem false :!label _label))
    (:`NewEnumerator1`
      (goto _label))
    (:`NewEnumerator2`
      (`PrimitiveComponent.SetSimulatePhysics` _totem true))
    (:`NewEnumerator3`
      (goto _label))))

(fn `UserConstructionScript`)