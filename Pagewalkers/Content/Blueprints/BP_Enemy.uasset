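; BP_Enemy is an enemy Blueprint with a health bar and target-lock widget that takes part in the player's turn-order system.
; On BeginPlay it caches BP_Player and has an event to rotate toward the player.
; Tick drives the health bar from EnemyHealth against a hard-coded maximum, and two events toggle the lock marker.
; A death check removes the enemy from the player's TurnOrderArray and Enemies lists.
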(event `self.ReceiveBeginPlay`
  (bind _asbp_player (cast `/Game/Blueprints/BP_Player` (`GameplayStatics.GetPlayerCharacter` 0)))
  (set `self.Player` _asbp_player)
  (`self.Set Enemy Rotation`))

(event `Set Enemy Rotation`
  (`self.K2_SetActorRotation` self (`KismetMathLibrary.FindLookAtRotation` (`self.K2_GetActorLocation` self) (`self.K2_GetActorLocation` (`self.Player`))) false))

(event `self.ReceiveTick`
  (params (DeltaSeconds :type "Float (single-precision)"))
  (bind _aswd_enemy_health_bar (cast `/Game/Blueprints/WD_EnemyHealthBar` (`WidgetComponent.GetWidget` (`self.WD_EnemyHealthBar`))))
  (set `ProgressBar.Percent` (/ (`self.EnemyHealth`) 500.0) (`/Game/Blueprints/WD_EnemyHealthBar.EnemyHealthBar` _aswd_enemy_health_bar)))

(event `SetEnemyTargetLockVisibility1`
  (`SceneComponent.SetVisibility` (`self.WD_TargetLock`) true false))

(event `SetEnemyTargetLockVisibility0`
  (`SceneComponent.SetVisibility` (`self.WD_TargetLock`) false false))

(event `CheckIfEnemyIsDead`
  (if (`self.EnemyDied`)
    (`KismetArrayLibrary.Array_RemoveItem` (`/Game/Blueprints/BP_Player.TurnOrderArray` (`self.Player`)) self)
    (`KismetArrayLibrary.Array_RemoveItem` (`/Game/Blueprints/BP_Player.Enemies` (`self.Player`)) self)))

(fn `UserConstructionScript`)