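; BP_Enemy is an enemy actor that turns to face the player when play begins.
; BeginPlay casts the first player character to BP_Player, stores it, then calls the SetEnemyRotation event.
; That event applies the full look-at rotation from the enemy to the player as a single snap, with no per-frame update in this graph.
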(event `self.ReceiveBeginPlay`
  (bind _asbp_player (cast `/Game/ThirdPerson/Blueprints/BP_Player` (`GameplayStatics.GetPlayerCharacter` 0)))
  (set `self.Player` _asbp_player)
  (`self.Set Enemy Rotation`))

(event `Set Enemy Rotation`
  (`self.K2_SetActorRotation` self (`KismetMathLibrary.FindLookAtRotation` (`self.K2_GetActorLocation` self) (`self.K2_GetActorLocation` (`self.Player`))) false))

(fn `UserConstructionScript`)